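; BP_PathFollower is an actor with a Brutum skeletal mesh that starts a kill sequence when the player character overlaps its Box.
; The overlap sets IsKilling on the mesh's ABP_Brutum anim instance, and Tick then raises its TransitionInt every frame.
; When the anim instance's ShouldCameraActivate is set during the kill, Tick blends the player's view to this actor and clears the flag.
; No path-following logic is present.
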(event OnComponentBeginOverlap(Box)
  (params (OverlappedComponent :type Primitive%20Component%20Object%20Reference) (OtherActor :type Actor%20Object%20Reference) (OtherComp :type Primitive%20Component%20Object%20Reference) (OtherBodyIndex :type Integer) (bFromSweep :type Boolean) (SweepResult :type Hit%20Result%20Structure%20%28by%20ref%29))
  (if (== OtherActor (Variables|Default|GetAs%20BP%20Controllable%20Character))
    (Variables|/Game/Animation/ABP_Brutum.ABP_Brutum_C|SetIsKilling (Variables|Default|GetAs%20ABP%20Brutum) true)))

(event EventBeginPlay
  (bind _asbp_controllable_character (Utilities|Casting|CastToBP_ControllableCharacter (Game|Player|GetPlayerPawn 0)))
  (Variables|Default|SetAs%20BP%20Controllable%20Character _asbp_controllable_character)
  (bind _asabp_brutum (Utilities|Casting|CastToABP_Brutum (Components|SkeletalMesh|GetAnimInstance (Variables|Default|GetSkeletalMesh))))
  (Variables|Default|SetAs%20ABP%20Brutum _asabp_brutum))

(event Collision|EventActorBeginOverlap
  (params (OtherActor :type Actor%20Object%20Reference)))

(event EventTick
  (params (DeltaSeconds :type Float%20%28single-precision%29))
  (bind _as_abp_brutum (Variables|Default|GetAs%20ABP%20Brutum))
  (if (Variables|/Game/Animation/ABP_Brutum.ABP_Brutum_C|GetIsKilling _as_abp_brutum)
    (Variables|/Game/Animation/ABP_Brutum.ABP_Brutum_C|SetTransitionInt _as_abp_brutum (+ (Variables|/Game/Animation/ABP_Brutum.ABP_Brutum_C|GetTransitionInt _as_abp_brutum) 5))
    (if (Variables|/Game/Animation/ABP_Brutum.ABP_Brutum_C|GetShouldCameraActivate _as_abp_brutum)
      (Game|Player|SetViewTargetwithBlend (Game|GetPlayerController 0) self 1.0 "VTBlend_Linear" 0.0 false)
      (Variables|/Game/Animation/ABP_Brutum.ABP_Brutum_C|SetShouldCameraActivate _as_abp_brutum false))))

(fn ConstructionScript)