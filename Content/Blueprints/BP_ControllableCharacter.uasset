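; BP_ControllableCharacter is a player character that collects a BP_Mote to end the game.
; On BeginPlay it finds the mote in the level, caches a reference and enables input from player controller 0.
; IA_Interact destroys the mote if its ShowText flag is set, then after a one-second delay shows the UI_EndGame widget and the mouse cursor.
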(event Input|EnhancedActionEvents|EnhancedInputActionIA_Interact
  (params (ActionValue :type Boolean) (ElapsedSeconds :type Float%20%28double-precision%29) (TriggeredSeconds :type Float%20%28double-precision%29) (InputAction :type Input%20Action%20Object%20Reference :default "/Game/Input/IA_Interact.IA_Interact"))
  (bind _as_bp_mote (Variables|Default|GetAs%20BP%20Mote))
  (Utilities|IsValid _as_bp_mote
    (:Is%20Valid
      (if (Variables|/Game/Blueprints/BP_Mote.BP_Mote_C|GetShowText _as_bp_mote)
        (Actor|DestroyActor _as_bp_mote)
        (Utilities|FlowControl|Delay 1.0)
        (bind _returnvalue (UserInterface|CreateWidget "/Game/UI/UI_EndGame.UI_EndGame_C"))
        (UserInterface|Viewport|AddtoViewport _returnvalue 0)
        (Variables|/Script/Engine.PlayerController|SetbShowMouseCursor (Game|GetPlayerController 0) true)))))

(event EventBeginPlay
  (bind _returnvalue (Actor|GetActorOfClass "/Game/Blueprints/BP_Mote.BP_Mote_C"))
  (bind _asbp_mote (Utilities|Casting|CastToBP_Mote _returnvalue))
  (Variables|Default|SetAs%20BP%20Mote _asbp_mote)
  (Input|EnableInput (Game|GetPlayerController 0)))

(event Collision|EventActorBeginOverlap
  (params (OtherActor :type Actor%20Object%20Reference)))

(event EventTick
  (params (DeltaSeconds :type Float%20%28single-precision%29)))

(event Input|KeyboardEvents|E
  (params (Key :type Key%20Structure :default "None")))

(fn ConstructionScript)