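; BP_Mote is an actor that detects when the player is looking at it and records the result in a ShowText flag.
; Every tick it line-traces for WorldDynamic objects from the player pawn's location along the camera's forward vector, between the Value and Power distances.
; ShowText is true only when the trace hits this mote itself; any other hit or a miss clears it.
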(event Collision|EventActorBeginOverlap
  (params (OtherActor :type Actor%20Object%20Reference)))

(event EventTick
  (params (DeltaSeconds :type Float%20%28single-precision%29))
  (bind _returnvalue (Game|Player|GetPlayerPawn 0))
  (bind _returnvalue_2 (Game|GetPlayerController 0))
  (bind _returnvalue_3 (Transformation|GetActorLocation _returnvalue))
  (bind _playercameramanager (Variables|/Script/Engine.PlayerController|GetPlayerCameraManager _returnvalue_2))
  (bind _returnvalue_4 (Camera|GetCameraRotation _playercameramanager))
  (bind _returnvalue_5 (Math|Vector|GetForwardVector _returnvalue_4))
  (bind (_outhit _returnvalue_6) (Collision|LineTraceForObjects (+ _returnvalue_3 (* _returnvalue_5 (Variables|Default|GetValue))) (+ _returnvalue_3 (* _returnvalue_5 (Variables|Default|GetPower))) (Utilities|Array|MakeArray "ObjectTypeQuery2") false 0 "None" false))
  (if _returnvalue_6
    (if (== (.HitActor (Collision|BreakHitResult _outhit)) self)
      (Variables|Default|SetShowText true)
      (else
        (Variables|Default|SetShowText false :!label _label)))
    (else
      (goto _label))))

(fn ConstructionScript)